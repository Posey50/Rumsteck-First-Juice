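; BP_End is a level-end trigger actor that shows the win screen when the player character reaches it.
; On overlap with BP_ThirdPersonCharacter it disables pausing on that character, creates WBP_WinMenu and adds it to the viewport with its FadeInWin animation.
; It then shows the mouse cursor for the first player controller and destroys itself.
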(event `self.ReceiveActorBeginOverlap`
  (params (OtherActor :type "Actor Object Reference"))
  (bind _ui_win (`self.UI_Win`))
  (bind _asbp_third_person_character (cast `/Game/ThirdPerson/Blueprints/BP_ThirdPersonCharacter` OtherActor))
  (set `/Game/ThirdPerson/Blueprints/BP_ThirdPersonCharacter.CanPause` false _asbp_third_person_character)
  (bind _returnvalue (`|CreateWidget` "/Game/Workshop/Blueprints/UI/WBP_WinMenu.WBP_WinMenu_C"))
  (bind _output_get (set `self.UI_Win` _returnvalue))
  (`UserWidget.AddToViewport` _output_get 0)
  (`UserWidget.PlayAnimation` _ui_win (`/Game/Workshop/Blueprints/UI/WBP_WinMenu.FadeInWin` _ui_win) 0.0 1 "Forward" 1.0 false)
  (set `PlayerController.bShowMouseCursor` true (`GameplayStatics.GetPlayerController` 0))
  (`self.K2_DestroyActor`))

(fn `UserConstructionScript`)