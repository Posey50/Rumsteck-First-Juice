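; BP_Mine is a prop mine that damages a matching actor that overlaps it, then explodes and removes itself.
; On overlap, it checks the other actor's class against ClassToShoot, applies DamageAmount, calls PlayExplosion and destroys itself.
; PlayExplosion spawns the explosion emitter at the mine's location but plays the sound at the world origin.
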(event `self.ReceiveActorBeginOverlap`
  (params (OtherActor :type "Actor Object Reference"))
  (if (`KismetMathLibrary.ClassIsChildOf` (`GameplayStatics.GetObjectClass` OtherActor) (`self.ClassToShoot`))
    (`GameplayStatics.ApplyDamage` OtherActor (`self.DamageAmount`))
    (`self.PlayExplosion`)
    (`self.K2_DestroyActor`)))

(event `PlayExplosion`
  (`GameplayStatics.SpawnEmitterAtLocation` (`self.ExplosionVFX`) (`self.K2_GetActorLocation`))
  (`GameplayStatics.PlaySoundAtLocation` (`self.ExplosionSound`) (0.0 0.0 0.0) (struct) 1.0 1.0 0.0 null null null null))

(fn `UserConstructionScript`)