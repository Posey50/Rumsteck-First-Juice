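; BP_Enemy_2 is an enemy Blueprint that continuously aims at the player character.
; On BeginPlay it runs the parent logic and sets the projectile class to BP_RadisProjectile.
; Each Tick, after the parent's, it yaws the static mesh toward the player and pitches the gun mesh using look-at rotations from the actor's location, splitting aim across the two components.
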(event `self.ReceiveBeginPlay`
  (`parent.ReceiveBeginPlay`)
  (set `self.ProjectileClass` "/Game/Workshop/Blueprints/Projectiles/BP_RadisProjectile.BP_RadisProjectile_C"))

(event `self.ReceiveTick`
  (params (DeltaSeconds :type "Float (single-precision)"))
  (bind _gunmesh (`self.GunMesh`))
  (bind (_returnvalue_roll _returnvalue_pitch _returnvalue_yaw) (`KismetMathLibrary.BreakRotator` (`KismetMathLibrary.FindLookAtRotation` (`self.K2_GetActorLocation`) (`self.K2_GetActorLocation` (`GameplayStatics.GetPlayerCharacter` 0)))))
  (bind (_returnvalue_roll_2 _returnvalue_pitch_2) (`KismetMathLibrary.BreakRotator` (`KismetMathLibrary.FindLookAtRotation` (`self.K2_GetActorLocation` (`ActorComponent.GetOwner` (`self.GunMesh`))) (`self.K2_GetActorLocation` (`GameplayStatics.GetPlayerCharacter` 0)))))
  ;[1 1 1] Suit la position du joueur
  (`parent.ReceiveTick` DeltaSeconds)
  (`SceneComponent.K2_SetWorldRotation` (`self.StaticMesh`) (`KismetMathLibrary.MakeRotator` 0.0 0.0 _returnvalue_yaw) false false)
  (`SceneComponent.K2_SetRelativeRotation` _gunmesh (`KismetMathLibrary.MakeRotator` (.roll (`SceneComponent.RelativeRotation` _gunmesh)) _returnvalue_pitch_2 (.yaw (`SceneComponent.RelativeRotation` _gunmesh))) false false))

(fn `UserConstructionScript`)