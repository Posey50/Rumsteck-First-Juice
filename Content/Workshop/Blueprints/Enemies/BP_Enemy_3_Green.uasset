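; BP_Enemy_3_Green is an enemy variant that patrols back and forth along the world Y axis around its spawn point.
; BeginPlay records the starting Y and sets the inherited projectile class to BP_BrocoProjectile.
; Each Tick moves it by MoveSpeed without delta-time scaling and flips that speed once it reaches MoveRange on either side.
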(event `self.ReceiveBeginPlay`
  (bind (_returnvalue_x _returnvalue_y) (`KismetMathLibrary.BreakVector` (`self.K2_GetActorLocation`)))
  (`parent.ReceiveBeginPlay`)
  (set `self.StartPos` _returnvalue_y)
  (set `self.ProjectileClass` "/Game/Workshop/Blueprints/Projectiles/BP_BrocoProjectile.BP_BrocoProjectile_C"))

(event `self.ReceiveTick`
  (params (DeltaSeconds :type "Float (single-precision)"))
  (bind _returnvalue (`self.GetTransform`))
  (`parent.ReceiveTick` DeltaSeconds)
  (`self.K2_SetActorTransform` (`KismetMathLibrary.MakeTransform` (`KismetMathLibrary.MakeVector` (.x (.location _returnvalue)) (+ (.y (.location _returnvalue)) (`self.MoveSpeed`)) (.z (.location _returnvalue)))))
  (if (or (>= (.y (.location (`self.GetTransform`))) (+ (`self.StartPos`) (`self.MoveRange`))) (<= (.y (.location (`self.GetTransform`))) (- (`self.StartPos`) (`self.MoveRange`))))
    (set `self.MoveSpeed` (* (`self.MoveSpeed`) -1.0))))

(fn `UserConstructionScript`
  (`parent.UserConstructionScript`))