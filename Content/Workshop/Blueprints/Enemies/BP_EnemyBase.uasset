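; Base enemy Blueprint that fires projectiles at the player within range and dies when its health runs out.
; A looping timer set on BeginPlay calls Shoot, which, if shooting is enabled and the player is close enough, spawns a projectile at a socket with a configurable speed.
; A bound any-damage handler subtracts health, and Kill spawns a destruction effect before destroying the actor.
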(event `OnTakeAnyDamage_Event` :!signature `self.OnTakeAnyDamage`
  (params (DamagedActor :type "Actor Object Reference") (Damage :type "Float (single-precision)") (DamageType :type "DamageType Object Reference") (InstigatedBy :type "Controller Object Reference") (DamageCauser :type "Actor Object Reference"))
  ;[1 1 1] Applique les dommages subits
  (bind _output_get (set `self.Health` (- (`self.Health`) Damage)))
  (if (<= _output_get 0.0)
    (`self.Kill`)))

(event `self.ReceiveBeginPlay`
  ;[1 1 1] Timer déclenchant le shoot à intervale réguliere
  (`KismetSystemLibrary.K2_SetTimerDelegate` (delegate `Shoot`) (`self.ShootFrequency`) true)
  (add `self.OnTakeAnyDamage` (delegate `OnTakeAnyDamage_Event`)))

(event `Shoot`
  (if (and (`self.bShootEnabled`) (<= (`self.GetDistanceTo` (`GameplayStatics.GetPlayerCharacter` 0) self) (`self.RadiusToShoot`)))
    ;[1 1 1] On spawn le projectile
    (`|SpawnActorFromClass` (`self.ProjectileClass`) (`SceneComponent.K2_GetComponentToWorld` (`self.ProjectileSocket`)) "Undefined" "OverrideRootScale" null (`self.ProjectileSpeed`) null)))

(event `Kill`
  ;[1 1 1] Spawn une explosion
  (`GameplayStatics.SpawnEmitterAtLocation` (`self.DestructionVFX`) (`self.K2_GetActorLocation`) (struct) (3.0 3.0 3.0))
  ;[1 1 1] Detruit l'ennemi
  (`self.K2_DestroyActor`))

(fn `UserConstructionScript`)