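; BP_Lardon_Projectile is a projectile that damages actors of a configurable target class and destroys itself on overlap.
; The construction script feeds the InitialSpeed variable into its projectile movement component.
; Any overlap calls ProjectileHit, which applies damage only if the touched actor derives from ClassToShot.
; It then always plays the explosion emitter and sound through HitEffect before being destroyed, regardless of what it touched.
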(event `self.ReceiveActorBeginOverlap`
  (params (OtherActor :type "Actor Object Reference"))
  (`self.ProjectileHit` OtherActor))

(event `ProjectileHit`
  (params (ActorTouched :type "Actor Object Reference"))
  (if (`KismetMathLibrary.ClassIsChildOf` (`GameplayStatics.GetObjectClass` ActorTouched) (`self.ClassToShot`))
    (`GameplayStatics.ApplyDamage` ActorTouched (`self.Damage`)))
  (`self.HitEffect`)
  (`self.K2_DestroyActor`))

(fn `HitEffect`
  (bind _returnvalue (`self.K2_GetActorLocation`))
  (`GameplayStatics.SpawnEmitterAtLocation` (`self.ExplosionVFX`) _returnvalue)
  (`GameplayStatics.PlaySoundAtLocation` (`self.SoundExplosion`) _returnvalue (struct) 1.0 1.0 0.0 null null null null))

(fn `UserConstructionScript`
  (set `ProjectileMovementComponent.InitialSpeed` (`self.InitialSpeed`) (`self.ProjectileMovement`)))