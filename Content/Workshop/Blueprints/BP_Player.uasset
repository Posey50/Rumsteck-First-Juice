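; Player pawn with forward/turn movement, health, two projectile weapons and a HUD widget created on BeginPlay.
; Each shot checks optional ammo and a cooldown, then spawns its projectile at ProjectileSocket, adding player speed to Shoot1Speed (used by both weapons) so the player cannot outrun it.
; Damage lowers health until death spawns an explosion and destroys the actor.
; AddHealth, AddAmmo1 and AddAmmo2 refill values, clamped to their maximums.
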(event `self.ReceiveBeginPlay`
  (add `self.OnTakeAnyDamage` (delegate `OnTakeAnyDamage_Event`))
  (bind _returnvalue (`|CreateWidget` "/Game/Workshop/Blueprints/UI/WBP_PlayerHUD.WBP_PlayerHUD_C" null self))
  (`UserWidget.AddToViewport` _returnvalue 0)
  (set `self.Shoot1_Ammo` (`self.Shoot1_MaxAmmo`))
  (set `self.Shoot2_Ammo` (`self.Shoot2_MaxAmmo`))
  (set `self.Health` (`self.MaxHealth`)))

(event `OnTakeAnyDamage_Event` :!signature `self.OnTakeAnyDamage`
  (params (DamagedActor :type "Actor Object Reference") (Damage :type "Float (single-precision)") (DamageType :type "DamageType Object Reference") (InstigatedBy :type "Controller Object Reference") (DamageCauser :type "Actor Object Reference"))
  ;[1 0.234 0.5197] Applique les dégats
  (bind _output_get (set `self.Health` (- (`self.Health`) Damage)))
  (if (<= _output_get 0.0)
    (`self.Dead`)))

(event `InputAxis|Forward`
  (params (AxisValue :type "Float (single-precision)"))
  ;[0.2089 1 0.1844] Mouvements
  ;;[1 1 1] Avance et recule
  (`self.AddMovementInput` (`self.GetActorForwardVector`) AxisValue))

(event `InputAction|PrimaryShoot`
  (params (Key :type "Key Structure"))
  ;[1 0.4873 0.4574] Shoots
  (:`Pressed`
    ;;[1 1 1] Check Ammo
    (if (`self.bShoot1_NeedAmmo`)
      (if (> (`self.Shoot1_Ammo`) 0)
        ;;[1 1 1] Check cooldown
        (if (>= (- (`GameplayStatics.GetTimeSeconds`) (`self.Shoot1_LastTime`)) (`self.Shoot1_Cooldown`)) :!label _label
          (set `self.Shoot1_LastTime` (`GameplayStatics.GetTimeSeconds`))
          ;;[1 1 1] On spawn le projectile
          (`|SpawnActorFromClass` "/Game/Workshop/Blueprints/Projectiles/BP_BaseProjectile.BP_BaseProjectile_C" (`SceneComponent.K2_GetComponentToWorld` (`self.ProjectileSocket`)) "Undefined" "OverrideRootScale" null (+ (`self.Shoot1_Speed`) (`KismetMathLibrary.VSize` (`self.GetVelocity`))) null)
          (set `self.Shoot1_Ammo` (`KismetMathLibrary.Clamp` (- (`self.Shoot1_Ammo`) 1) 0 (`self.Shoot1_MaxAmmo`)))))
      (else
        (goto _label)))))

(event `InputAxis|Turn`
  (params (AxisValue :type "Float (single-precision)"))
  ;[0.2089 1 0.1844] Mouvements
  ;;[1 1 1] Mouvement de rotation
  (`self.AddControllerYawInput` AxisValue))

(event `InputAction|SecondaryShoot`
  (params (Key :type "Key Structure"))
  ;[1 0.4873 0.4574] Shoots
  (:`Pressed`
    ;;[1 1 1] Check Ammo
    (if (`self.bShoot2_NeedAmmo`)
      (if (> (`self.Shoot2_Ammo`) 0)
        ;;[1 1 1] Check cooldown
        (if (>= (- (`GameplayStatics.GetTimeSeconds`) (`self.Shoot2_LastTime`)) (`self.Shoot2_Cooldown`)) :!label _label_2
          (set `self.Shoot2_LastTime` (`GameplayStatics.GetTimeSeconds`))
          ;;[1 1 1] On spawn le projectile
          (`|SpawnActorFromClass` "/Game/Workshop/Blueprints/Projectiles/BP_LargeProjectile.BP_LargeProjectile_C" (`SceneComponent.K2_GetComponentToWorld` (`self.ProjectileSocket`)) "Undefined" "OverrideRootScale" null (+ (`self.Shoot1_Speed`) (`KismetMathLibrary.VSize` (`self.GetVelocity`))) null)
          (set `self.Shoot2_Ammo` (`KismetMathLibrary.Clamp` (- (`self.Shoot2_Ammo`) 1) 0 (`self.Shoot2_MaxAmmo`)))))
      (else
        (goto _label_2)))))

(event `AddAmmo1`
  (params (Amount :type Integer))
  ;[0.4948 0.4948 0.4948] ajoute des munitions
  (set `self.Shoot1_Ammo` (`KismetMathLibrary.Clamp` (+ Amount (`self.Shoot1_Ammo`)) 0 (`self.Shoot1_MaxAmmo`))))

(event `AddHealth`
  (params (Amount :type "Float (double-precision)"))
  ;[0 1 0.04119] Ajoute de la santé
  (set `self.Health` (`KismetMathLibrary.FClamp` (+ Amount (`self.Health`)) 0.0 (`self.MaxHealth`))))

(event `Dead`
  ;[1 1 1] Mort du joueur
  (`GameplayStatics.SpawnEmitterAtLocation` "/Game/StarterContent/Particles/P_Explosion.P_Explosion" (`self.K2_GetActorLocation`) (struct) (3.0 3.0 3.0))
  (`self.K2_DestroyActor`))

(event `AddAmmo2`
  (params (Amount :type Integer))
  ;[0.4948 0.4948 0.4948] ajoute des munitions
  (set `self.Shoot2_Ammo` (`KismetMathLibrary.Clamp` (+ Amount (`self.Shoot2_Ammo`)) 0 (`self.Shoot2_MaxAmmo`))))

(fn `UserConstructionScript`)